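; BP_PatrolEnemy is an enemy actor that moves between two target points along the world Y axis.
; On BeginPlay, if both points are non-zero, it plays the PatrolMovement timeline with MovementSpeed as the play rate.
; Each update lerps between the points by the timeline alpha and applies only the Y component, without sweeping, keeping current X and Z.
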(event `self.ReceiveBeginPlay`
  (if (and (!= (`self.TargetPoint_A`) (0.0 0.0 0.0)) (!= (`self.TargetPoint_B`) (0.0 0.0 0.0)))
    (`TimelineComponent.SetPlayRate` (`self.PatrolMovement`) (`self.MovementSpeed`))
    (bind (_direction _patrolalpha) (`Timeline|PatrolMovement`)
      (:`Update`
        (`self.K2_SetActorLocation` (`KismetMathLibrary.MakeVector` (.x (`self.K2_GetActorLocation`)) (.y (`KismetMathLibrary.VLerp` (`self.TargetPoint_A`) (`self.TargetPoint_B`) _patrolalpha)) (.z (`self.K2_GetActorLocation`))))))))

(fn `UserConstructionScript`)