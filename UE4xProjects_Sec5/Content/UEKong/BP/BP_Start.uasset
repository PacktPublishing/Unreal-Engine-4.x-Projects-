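; Level start countdown actor that shows the seconds left on a text display, then signals the player character that the game has started.
; BeginPlay starts a one-shot four-second timer, and Tick runs TimeToGo every frame to display that timer's floored remaining time.
; Once TimeLeft reaches zero, TimeToGo shows "START!" and calls CallGameHasStarted on the SideScrollerCharacter, repeating on subsequent ticks.
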(event `self.ReceiveBeginPlay`
  (bind _returnvalue (`KismetSystemLibrary.K2_SetTimerDelegate` (delegate `TimeToGo`) 4.0)))

(event `TimeToGo`
  (if (<= (`self.TimeLeft`) 0)
    (`TextRenderComponent.K2_SetText` (`self.CountDownText`) (`KismetTextLibrary.Conv_StringToText` "START!"))
    (bind _asside_scroller_character (cast `/Game/SideScrollerBP/Blueprints/SideScrollerCharacter` (`GameplayStatics.GetPlayerCharacter` 0)))
    (`/Game/SideScrollerBP/Blueprints/SideScrollerCharacter.GameHasStarted` _asside_scroller_character)
    (else
      (bind _output_get (set `self.TimeLeft` (`KismetMathLibrary.FFloor` (`KismetSystemLibrary.K2_GetTimerRemainingTimeHandle` (stale `self.ReceiveBeginPlay` _returnvalue)))))
      (`TextRenderComponent.K2_SetText` (`self.CountDownText`) (`KismetTextLibrary.Conv_IntToText` _output_get)))))

(event `self.ReceiveTick`
  (params (DeltaSeconds :type "Float (single-precision)"))
  (`self.TimeToGo`))

(fn `UserConstructionScript`)