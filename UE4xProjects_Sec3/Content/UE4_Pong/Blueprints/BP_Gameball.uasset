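; BP_Gameball is the Pong ball, launched along the Y axis by setting its physics velocity on BeginPlay.
; Overlaps drive bouncing: paddles reverse Y, pass their own X velocity to the ball and increment a volley count, while boundaries reverse X.
; Goals trigger an explosion, then spawn a replacement ball at the origin, with direction set by the goal hit, and destroy this one.
; Scoring, reset and quit logic is present but disconnected.
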(event `self.ReceiveBeginPlay`
  (`PrimitiveComponent.SetPhysicsLinearVelocity` (`self.StaticMeshComponent`) (0.0 -1000.0 0.0) false "None"))

(event `self.ReceiveActorBeginOverlap`
  (params (OtherActor :type "Actor Object Reference"))
  (bind _volleycount (`self.VolleyCount`))
  (bind _staticmeshcomponent (`self.StaticMeshComponent`))
  (bind _staticmeshcomponent_2 (`self.StaticMeshComponent`))
  (bind _returnvalue (`SceneComponent.K2_GetComponentLocation` (`self.StaticMeshComponent`)))
  (bind _asbp_paddle_p1 (cast `/Game/UE4_Pong/Blueprints/BP_Paddle_P1` OtherActor)
    (:`then`
      (bind _returnvalue_2 (`PrimitiveComponent.GetPhysicsLinearVelocity` (`/Game/UE4_Pong/Blueprints/BP_Paddle_P1.SM_Paddle` _asbp_paddle_p1) "None"))
      (`KismetSystemLibrary.PrintString` "HIT" true true (struct :`R` 0.121183 :`G` 1.0 :`B` 0.020612 :`A` 1.0))
      (bind _returnvalue_3 (`PrimitiveComponent.GetPhysicsLinearVelocity` _staticmeshcomponent_2 "None"))
      (`PrimitiveComponent.SetPhysicsLinearVelocity` _staticmeshcomponent_2 (`KismetMathLibrary.MakeVector` (.x _returnvalue_2) (* (.y _returnvalue_3) -1.0) (.z _returnvalue_3)) false "None")
      ;[1 1 1] VolleyCountForMultiball
      (`/Engine/EditorBlueprintResources/StandardMacros.IncrementInt` _volleycount :!label _label
        (:`  `
          (`KismetSystemLibrary.PrintString` (`KismetStringLibrary.Conv_IntToString` _volleycount) true true (struct :`R` 1.0 :`G` 0.012887 :`B` 0.739153 :`A` 1.0)))))
    (:`CastFailed`
      (cast `/Game/UE4_Pong/Blueprints/BP_Boundary_Blueprint` OtherActor
        (:`then`
          (`KismetSystemLibrary.PrintString` "HIT" true true (struct :`R` 0.121183 :`G` 1.0 :`B` 0.020612 :`A` 1.0))
          (bind _returnvalue_4 (`PrimitiveComponent.GetPhysicsLinearVelocity` _staticmeshcomponent_2 "None"))
          (`PrimitiveComponent.SetPhysicsLinearVelocity` _staticmeshcomponent_2 (`KismetMathLibrary.MakeVector` (* (.x _returnvalue_4) -1.0) (.y _returnvalue_4) (.z _returnvalue_4)) false "None"))
        (:`CastFailed`
          (bind _asbp_paddle_ai (cast `/Game/UE4_Pong/Blueprints/BP_Paddle_AI` OtherActor)
            (:`then`
              (bind _returnvalue_5 (`PrimitiveComponent.GetPhysicsLinearVelocity` (`/Game/UE4_Pong/Blueprints/BP_Paddle_AI.SM_Paddle` _asbp_paddle_ai) "None"))
              (`KismetSystemLibrary.PrintString` "HIT" true true (struct :`R` 0.121183 :`G` 1.0 :`B` 0.020612 :`A` 1.0))
              (bind _returnvalue_6 (`PrimitiveComponent.GetPhysicsLinearVelocity` _staticmeshcomponent "None"))
              (`PrimitiveComponent.SetPhysicsLinearVelocity` _staticmeshcomponent (`KismetMathLibrary.MakeVector` (.x _returnvalue_5) (* (.y _returnvalue_6) -1.0) (.z _returnvalue_6)) false "None")
              (goto _label))
            (:`CastFailed`
              (cast `/Game/UE4_Pong/Blueprints/BP_GoalLeft` OtherActor
                (:`then`
                  (`GameplayStatics.SpawnEmitterAtLocation` "/Game/StarterContent/Particles/P_Explosion.P_Explosion" _returnvalue)
                  (`KismetSystemLibrary.Delay` 0.5)
                  (`self.CPU_Spawn`))
                (:`CastFailed`
                  (cast `/Game/UE4_Pong/Blueprints/BP_GoalRight` OtherActor)
                  (`GameplayStatics.SpawnEmitterAtLocation` "/Game/StarterContent/Particles/P_Explosion.P_Explosion" _returnvalue)
                  (`KismetSystemLibrary.Delay` 0.5)
                  (`self.P1_Spawn`)))
              (`self.K2_DestroyActor`))))))))

(event `P1_Spawn`
  (bind _returnvalue (`|SpawnActorFromClass` "BP_Gameball_C" (`KismetMathLibrary.MakeTransform` (0.0 0.0 0.0)) "Undefined" "OverrideRootScale"))
  (bind _staticmeshcomponent (`StaticMeshActor.StaticMeshComponent` _returnvalue))
  (bind _returnvalue_2 (`PrimitiveComponent.GetPhysicsLinearVelocity` _staticmeshcomponent "None"))
  (`PrimitiveComponent.SetPhysicsLinearVelocity` _staticmeshcomponent (* _returnvalue_2 -1.0) false "None"))

(event `CPU_Spawn`
  (`|SpawnActorFromClass` "BP_Gameball_C" (`KismetMathLibrary.MakeTransform` (0.0 0.0 0.0)) "Undefined" "OverrideRootScale"))

(fn `UserConstructionScript`)