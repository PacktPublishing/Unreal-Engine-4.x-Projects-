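; BP_LazerBox_byObject is an actor that periodically fires a visible debug laser downward along its local up axis, tracing for WorldDynamic objects.
; A latent Delay on Tick throttles the line trace to roughly every four seconds.
; A looping MultiGate alternates the hit component's material between red and blue on successive traces.
; A fire emitter spawns at the impact point, with no check that the trace hit anything.
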(event `self.ReceiveActorBeginOverlap`
  (params (OtherActor :type "Actor Object Reference")))

(event `self.ReceiveTick`
  (params (DeltaSeconds :type "Float (single-precision)"))
  (bind _returnvalue (`self.K2_GetActorLocation`))
  (`KismetSystemLibrary.Delay` 4.0)
  (bind _outhit (`KismetSystemLibrary.LineTraceSingleForObjects` :`Start` _returnvalue :`End` (+ _returnvalue (* (`self.GetActorUpVector`) -500.0)) :`ObjectTypes` (`|MakeArray` "ObjectTypeQuery2" :!type "EObjectTypeQuery Enum") :`DrawDebugType` "ForDuration" :`DrawTime` 2.0))
  (`|MultiGate` false true 0
    (:`Out 0`
      (bind (_bblockinghit _binitialoverlap _time _location _impactpoint _normal _impactnormal _physmat _hitactor _hitcomponent) (`GameplayStatics.BreakHitResult` _outhit))
      (`PrimitiveComponent.SetMaterial` _hitcomponent 0 "/Game/ImRed.ImRed"))
    (:`Out 1`
      (`PrimitiveComponent.SetMaterial` _hitcomponent 0 "/Game/ImBlue.ImBlue")))
  (`GameplayStatics.SpawnEmitterAtLocation` "/Game/StarterContent/Particles/P_Fire.P_Fire" _impactpoint))

(fn `UserConstructionScript`)