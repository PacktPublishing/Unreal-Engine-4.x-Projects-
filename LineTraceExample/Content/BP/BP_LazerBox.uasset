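; BP_LazerBox is an actor that periodically fires a debug-drawn line trace and recolors whatever component it hits.
; Tick feeds a Delay, so roughly every four seconds it traces a short distance along the actor's forward vector on the Visibility channel.
; A looping MultiGate alternates the hit component's material between ImRed and ImBlue, printing the matching color message, with no check that the trace hit.
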(event `self.ReceiveActorBeginOverlap`
  (params (OtherActor :type "Actor Object Reference")))

(event `self.ReceiveTick`
  (params (DeltaSeconds :type "Float (single-precision)"))
  (bind _returnvalue (`self.K2_GetActorLocation`))
  (`KismetSystemLibrary.Delay` 4.0)
  (bind _outhit (`KismetSystemLibrary.LineTraceSingle` :`Start` _returnvalue :`End` (+ _returnvalue (* (`self.GetActorForwardVector`) 500.0)) :`TraceChannel` "TraceTypeQuery1" :`DrawDebugType` "ForDuration" :`DrawTime` 2.0))
  (`|MultiGate` false true 0
    (:`Out 0`
      (`KismetSystemLibrary.PrintString` "I'm RED!")
      (bind (_bblockinghit _binitialoverlap _time _location _impactpoint _normal _impactnormal _physmat _hitactor _hitcomponent) (`GameplayStatics.BreakHitResult` _outhit))
      (`PrimitiveComponent.SetMaterial` _hitcomponent 0 "/Game/ImRed.ImRed"))
    (:`Out 1`
      (`KismetSystemLibrary.PrintString` "I'm BLUE!")
      (`PrimitiveComponent.SetMaterial` _hitcomponent 0 "/Game/ImBlue.ImBlue"))))

(fn `UserConstructionScript`)