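; Pong ball that launches along Y at start, bounces off paddles and boundaries, and keeps score for player and CPU.
; Overlap casts pick the response: paddles reverse Y velocity and pass on their own X velocity, boundaries reverse X.
; Goals increment and print the score, then after a delay recenter and relaunch the ball.
; The game quits once either side's score exceeds two.
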(event `self.ReceiveBeginPlay`
  ;[1 1 1] GameStarts!
  (`PrimitiveComponent.SetPhysicsLinearVelocity` (`self.StaticMeshComponent`) (0.0 -1000.0 0.0) false "None"))

(event `self.ReceiveActorBeginOverlap`
  (params (OtherActor :type "Actor Object Reference"))
  (bind _staticmeshcomponent (`self.StaticMeshComponent`))
  (bind _staticmeshcomponent_2 (`self.StaticMeshComponent`))
  ;[1 1 1] BallCollidesWith...
  ;[0 0.716 1] Player
  (bind _asbp_paddle_p1 (cast `/Game/UE4_Pong/Blueprints/BP_Paddle_P1` OtherActor)
    (:`then`
      (bind _returnvalue (`PrimitiveComponent.GetPhysicsLinearVelocity` (`/Game/UE4_Pong/Blueprints/BP_Paddle_P1.SM_Paddle` _asbp_paddle_p1) "None"))
      (`KismetSystemLibrary.PrintString` "HIT" true true (struct :`R` 0.121183 :`G` 1.0 :`B` 0.020612 :`A` 1.0))
      (bind _returnvalue_2 (`PrimitiveComponent.GetPhysicsLinearVelocity` _staticmeshcomponent_2 "None"))
      (`PrimitiveComponent.SetPhysicsLinearVelocity` _staticmeshcomponent_2 (`KismetMathLibrary.MakeVector` (.x _returnvalue) (* (.y _returnvalue_2) -1.0) (.z _returnvalue_2)) false "None"))
    (:`CastFailed`
      ;[1 1 1] Boundary
      (cast `/Game/UE4_Pong/Blueprints/BP_Boundary_Blueprint` OtherActor
        (:`then`
          (`KismetSystemLibrary.PrintString` "HIT" true true (struct :`R` 0.121183 :`G` 1.0 :`B` 0.020612 :`A` 1.0))
          (bind _returnvalue_3 (`PrimitiveComponent.GetPhysicsLinearVelocity` _staticmeshcomponent_2 "None"))
          (`PrimitiveComponent.SetPhysicsLinearVelocity` _staticmeshcomponent_2 (`KismetMathLibrary.MakeVector` (* (.x _returnvalue_3) -1.0) (.y _returnvalue_3) (.z _returnvalue_3)) false "None"))
        (:`CastFailed`
          ;[1 0.16 0.3272] AI
          (bind _asbp_paddle_ai (cast `/Game/UE4_Pong/Blueprints/BP_Paddle_AI` OtherActor)
            (:`then`
              (bind _returnvalue_4 (`PrimitiveComponent.GetPhysicsLinearVelocity` (`/Game/UE4_Pong/Blueprints/BP_Paddle_AI.SM_Paddle` _asbp_paddle_ai) "None"))
              (`KismetSystemLibrary.PrintString` "HIT" true true (struct :`R` 0.121183 :`G` 1.0 :`B` 0.020612 :`A` 1.0))
              (bind _returnvalue_5 (`PrimitiveComponent.GetPhysicsLinearVelocity` _staticmeshcomponent "None"))
              (`PrimitiveComponent.SetPhysicsLinearVelocity` _staticmeshcomponent (`KismetMathLibrary.MakeVector` (.x _returnvalue_4) (* (.y _returnvalue_5) -1.0) (.z _returnvalue_5)) false "None"))
            (:`CastFailed`
              ;[0.3227 0.59 0.2841] Goals
              (cast `/Game/UE4_Pong/Blueprints/BP_GoalLeft` OtherActor
                (:`then`
                  (bind _output_get (set `self.ScoreCPU` (+ (`self.ScoreCPU`) 1)))
                  (`KismetSystemLibrary.PrintString` (`KismetStringLibrary.Conv_IntToString` _output_get) true true (struct :`R` 1.0 :`G` 0.235508 :`B` 0.014647 :`A` 1.0))
                  (`KismetSystemLibrary.Delay` 0.5)
                  (`self.K2_SetActorLocation` (0.0 0.0 0.0))
                  (`PrimitiveComponent.SetPhysicsLinearVelocity` (`self.StaticMeshComponent`) (0.0 1000.0 0.0) false "None")
                  (if (> (`self.ScoreCPU`) 2)
                    (`KismetSystemLibrary.Delay` 1.0)
                    (`KismetSystemLibrary.QuitGame` null "Quit")))
                (:`CastFailed`
                  (cast `/Game/UE4_Pong/Blueprints/BP_GoalRight` OtherActor)
                  (bind _output_get_2 (set `self.ScorePlayer` (+ (`self.ScorePlayer`) 1)))
                  (`KismetSystemLibrary.PrintString` (`KismetStringLibrary.Conv_IntToString` _output_get_2) true true (struct :`R` 0.014152 :`G` 0.738004 :`B` 1.0 :`A` 1.0))
                  (`KismetSystemLibrary.Delay` 0.5)
                  (`self.K2_SetActorLocation` (0.0 0.0 0.0))
                  (`PrimitiveComponent.SetPhysicsLinearVelocity` (`self.StaticMeshComponent`) (0.0 -1000.0 0.0) false "None")
                  (if (> (`self.ScorePlayer`) 2)
                    (`KismetSystemLibrary.Delay` 1.0)
                    (`KismetSystemLibrary.QuitGame` null "Quit")))))))))))

(fn `UserConstructionScript`)