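; BP_Elevator is an elevator actor that moves vertically while a SideScrollerCharacter stands in its CanRide volume.
; It stores its starting Z on BeginPlay, then overlap begin plays the MovementControl timeline, whose UpDown track is added to that height each update.
; When the character leaves the volume, the timeline reverses, returning the elevator toward its origin.
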(event `self.ReceiveBeginPlay`
  (set `self.OriginLoc` (.z (`self.K2_GetActorLocation`))))

(event `self.CanRide.OnComponentBeginOverlap`
  (params (OverlappedComponent :type "PrimitiveComponent Object Reference") (OtherActor :type "Actor Object Reference") (OtherComp :type "PrimitiveComponent Object Reference") (OtherBodyIndex :type Integer) (bFromSweep :type Boolean) (SweepResult :type "HitResult Structure (by ref)"))
  (cast `/Game/SideScrollerBP/Blueprints/SideScrollerCharacter` OtherActor)
  (bind (_direction _updown) (`Timeline|MovementControl` :!label _label)
    (:`Update`
      (`self.K2_SetActorLocation` (`KismetMathLibrary.MakeVector` (.x (`self.K2_GetActorLocation`)) (.y (`self.K2_GetActorLocation`)) (+ _updown (`self.OriginLoc`)))))))

(event `self.CanRide.OnComponentEndOverlap`
  (params (OverlappedComponent :type "PrimitiveComponent Object Reference") (OtherActor :type "Actor Object Reference") (OtherComp :type "PrimitiveComponent Object Reference") (OtherBodyIndex :type Integer))
  (cast `/Game/SideScrollerBP/Blueprints/SideScrollerCharacter` OtherActor)
  (goto _label :!via `Reverse`))

(fn `UserConstructionScript`)